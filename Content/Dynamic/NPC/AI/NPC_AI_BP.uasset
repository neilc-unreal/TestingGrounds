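; AI controller for guard NPCs that runs the GuardBehaviour behavior tree on the PatrolData blackboard, both started at BeginPlay.
; AI Perception updates feed SetEnemyBasedOnPerception, which ignores actors tagged "Enemy" and stores any other sensed actor in the blackboard's enemy key.
; A failed or expired stimulus from such an actor clears that key.
; An unused debug helper prints sense results to screen.
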(event `self.ReceiveBeginPlay`
  (bind _blackboardcomponent (`self.UseBlackboard` "/Game/Dynamic/NPC/AI/PatrolData.PatrolData"))
  (`self.RunBehaviorTree` "/Game/Dynamic/NPC/AI/GuardBehaviour.GuardBehaviour")
  (set `self.BlackboardComp` _blackboardcomponent))

(event `self.ReceiveTick`
  (params (DeltaSeconds :type "Float (single-precision)")))

(event `self.AIPerception.OnTargetPerceptionUpdated`
  (params (Actor :type "Actor Object Reference") (Stimulus :type "AIStimulus Structure"))
  (`self.Set Enemy Based on Perception` Actor Stimulus))

(fn `Print Triggers To Screen`
  (params (Stimulus :type "AIStimulus Structure (by ref)") (Object :type "Object Object Reference"))
  (bind _returnvalue (`AIPerceptionSystem.GetSenseClassForStimulus` Stimulus))
  (`KismetSystemLibrary.PrintString` (`KismetStringLibrary.Concat_StrStr` (`KismetSystemLibrary.GetDisplayName` (`self.K2_GetPawn`)) " can " (`KismetSystemLibrary.GetClassDisplayName` _returnvalue) "(" (`KismetStringLibrary.Conv_BoolToString` (`.bSuccessfullySensed` (break `AIStimulus` Stimulus))) ")" (`KismetSystemLibrary.GetObjectName` Object))))

(fn `Set Enemy Based on Perception`
  (params (Actor :type "Actor Object Reference") (AIStimulus :type "AIStimulus Structure (by ref)"))
  (bind (_age _expirationage _strength _stimuluslocation _receiverlocation _tag _bsuccessfullysensed) (break `AIStimulus` AIStimulus))
  (bind _blackboardcomp (`self.BlackboardComp`))
  (bind _enemykey (`self.EnemyKey`))
  (if (`self.ActorHasTag` Actor "Enemy")
    _
    (elif (or (not _bsuccessfullysensed) (>= _age _expirationage))
      (`BlackboardComponent.ClearValue` _blackboardcomp _enemykey)
      (else
        (`BlackboardComponent.SetValueAsObject` _blackboardcomp _enemykey Actor)))))

(fn `UserConstructionScript`)