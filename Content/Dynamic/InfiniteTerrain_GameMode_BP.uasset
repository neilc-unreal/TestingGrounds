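; Game mode for an infinite terrain level that lays out the initial chain of Tile_BP actors on BeginPlay.
; It spawns a first tile behind the world origin along X, then loops to place each following tile at the previous tile's attach transform.
; SpawnTile stores and returns the newest tile as LastSpawnedTile, which anchors the next spawn.
; The ChoosePlayerStart override is empty and returns no start actor.
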(event `self.ReceiveBeginPlay`
  (`self.Spawn Tile` (`KismetMathLibrary.Conv_VectorToTransform` (-2000.0 0.0 0.0)))
  (for _ (range 10)
    (bind _attachlocation (`/Game/Dynamic/Terrain/Tile_BP.GetAttachLocation` (`self.LastSpawnedTile`)))
    (`self.Spawn Tile` _attachlocation)))

(fn `ChoosePlayerStart`
  (params (Player :type "Controller Object Reference"))
  (returns (ReturnValue :type "Actor Object Reference"))
  (return null))

(fn `Spawn Tile`
  (params (`At Location` :type "Transform Structure"))
  (returns (`Spawned Tile` :type "/Game/Dynamic/Terrain/Tile_BP Object Reference"))
  (bind _returnvalue (`|SpawnActorFromClass` "/Game/Dynamic/Terrain/Tile_BP.Tile_BP_C" `At Location` "Undefined" "OverrideRootScale"))
  (bind _output_get (set `self.LastSpawnedTile` _returnvalue))
  (return _output_get))

(fn `UserConstructionScript`)